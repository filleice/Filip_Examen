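; BP_GameplayLibrary is a Blueprint function library of static helpers for a gameplay-tag event system built on BP_EventSystemComponent.
; Each function looks up that component on a target actor.
; SendGameplayEvent forwards a tag, payload and optional object to it, and StartWaitingMultipleEvents registers a receiver for several tags, both skipping invalid lookups.
; GetEventComponent returns the component with a success flag.
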(fn SendGameplayEvent
  (params (Target :type Actor%20Object%20Reference) (Tag :type Gameplay%20Tag%20Structure) (Payload :type BP%20Payload%20Base%20Class%20Reference) (AdditionalObject :type Object%20Object%20Reference))
  (bind _returnvalue (Actor|GetComponentbyClass Target "/Game/_WhatYouPaidFor_RenameMe/Blueprints/Components/BP_EventSystemComponent.BP_EventSystemComponent_C"))
  (Utilities|IsValid Target
    (:Is%20Valid
      (Utilities|IsValid _returnvalue
        (:Is%20Valid
          (Default|ReceiveEvent _returnvalue Tag Payload AdditionalObject))))))

(fn StartWaitingMultipleEvents
  (params (Target :type Actor%20Object%20Reference) (EventReceiver :type Object%20Object%20Reference%20%28by%20ref%29) (Tags :type Gameplay%20Tag%20Container%20Structure))
  (bind _returnvalue (Actor|GetComponentbyClass Target "/Game/_WhatYouPaidFor_RenameMe/Blueprints/Components/BP_EventSystemComponent.BP_EventSystemComponent_C"))
  (Utilities|IsValid _returnvalue
    (:Is%20Valid
      (Default|WaitMultipleEvents _returnvalue EventReceiver Tags))))

(fn GetEventComponent
  (params (Target :type Actor%20Object%20Reference))
  (bind _returnvalue (Actor|GetComponentbyClass Target "/Game/_WhatYouPaidFor_RenameMe/Blueprints/Components/BP_EventSystemComponent.BP_EventSystemComponent_C"))
  (return (Utilities|IsValid _returnvalue) _returnvalue))