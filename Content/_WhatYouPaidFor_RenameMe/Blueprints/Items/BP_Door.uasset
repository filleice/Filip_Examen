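; Key-locked door that swings open when the player interacts while holding the matching key status tag.
; An interaction gameplay-tag event checks the tag, removes it from the player, marks the door open and starts RotatingMovement.
; Tick stops the rotation once a forward-vector dot product nears the saved target; the construction script previews that direction with a debug arrow.
; An overlap-driven TextRender prompts "Press E to Open", or "Find Key" without the key.
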(event OnComponentBeginOverlap(InteractTutorial)
  (params (OverlappedComponent :type Primitive%20Component%20Object%20Reference) (OtherActor :type Actor%20Object%20Reference) (OtherComp :type Primitive%20Component%20Object%20Reference) (OtherBodyIndex :type Integer) (bFromSweep :type Boolean) (SweepResult :type Hit%20Result%20Structure%20%28by%20ref%29))
  ;[1 1 1] Tutorial: Press E to Open
  (if (CallFunction|ShouldShowTutorial OtherActor)
    (CallFunction|ToggleTextRender false)))

(event OnComponentEndOverlap(InteractTutorial)
  (params (OverlappedComponent :type Primitive%20Component%20Object%20Reference) (OtherActor :type Actor%20Object%20Reference) (OtherComp :type Primitive%20Component%20Object%20Reference) (OtherBodyIndex :type Integer))
  ;[1 1 1] Tutorial: Press E to Open
  (if (== (Game|GetPlayerCharacter 0) OtherActor)
    (CallFunction|ToggleTextRender true)))

(event EventBeginPlay
  (CallFunction|SaveTargetRotaion)
  (Default|WaitMultipleEvents (Variables|Default|GetBP_EventSystemComponent) self "(GameplayTags=((TagName=\"Gameplay.Interraction\")))")
  (CallFunction|ToggleTextRender true))

(event EventTick
  (params (DeltaSeconds :type Float%20%28single-precision%29))
  ;[1 1 1] Opening door "Animation". I use RotatingMovementComponent (Unreal's)
  (if (>= (Math|Vector|DotProduct (Math|Vector|GetForwardVector (Variables|Door|Settings|GetTargetRotation)) (Transformation|GetActorForwardVector)) 0.99)
    (Components|Activation|Deactivate (Variables|Default|GetRotatingMovement))))

(event EventEvent
  (params (Tag :type Gameplay%20Tag%20Structure) (Payload :type BP%20Payload%20Base%20Class%20Reference) (OptionalObject :type Object%20Object%20Reference))
  (|SwitchGameplayTag Tag
    (:Gameplay.Interraction
      (CallFunction|ToggleTextRender true)
      (if (CallFunction|HasStatusTag (Game|GetPlayerCharacter 0) (Variables|Door|Settings|GetKeyTag) true)
        ;[1 1 1] StartOpeningDoor
        (Components|Activation|Activate (Variables|Default|GetRotatingMovement) false)
        (Actor|Tick|SetActorTickEnabled true)
        (CallFunction|ApplyStatustoActor self true "(TagName=\"Status.Door.Open\")")
        (CallFunction|ApplyStatustoActor (Game|GetPlayerCharacter 0) false (Variables|Door|Settings|GetKeyTag))
        (else
          ;[1 1 1] Find Key Tutorial
          (CallFunction|ToggleTextRender false)
          (Rendering|Components|TextRender|SetText (Variables|Default|GetTextRender) (Utilities|Text|MakeLiteralText "Find Key")))))))

(fn ConstructionScript
  (Rendering|Debug|FlushPersistentDebugLines)
  (Rendering|Debug|DrawDebugArrow (Transformation|GetActorLocation) (+ (Transformation|GetActorLocation) (* (Math|Vector|Normalize (Math|Vector|GetForwardVector (Math|Rotator|CombineRotators (Variables|Door|Settings|GetTargetRotation) (Transformation|GetActorRotation)))) 5e+02)) 1e+01 "(R=0.457271,G=0.000000,B=1.000000,A=1.000000)" 5e+03 5.0))

(fn ToggleTextRender
  (params (NewHidden :type Boolean))
  (Rendering|Components|TextRender|SetText (Variables|Default|GetTextRender) (Utilities|Text|MakeLiteralText "Press E to Open"))
  (Development|SetHiddeninGame (Variables|Default|GetTextRender) NewHidden false))

(fn SaveTargetRotaion
  (Variables|Door|Settings|SetTargetRotation (Math|Rotator|CombineRotators (Transformation|GetActorRotation) (Variables|Door|Settings|GetTargetRotation))))

(fn ShouldShowTutorial
  (params (Actor :type Object%20Object%20Reference))
  (return (and (== (Game|GetPlayerCharacter 0) Actor) (not (CallFunction|HasStatusTag self "(TagName=\"Status.Door.Open\")" true)))))