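; BP_Projectile is a projectile actor that flies toward the player and reports hits through a gameplay event.
; On BeginPlay it points the ProjectileMovement velocity at player pawn 0's current position using the initial speed, with no later re-aiming.
; When its Box overlaps any actor except its owner, it sends that actor a HitByProjectile event with an arrow damage payload, then destroys itself.
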(event OnComponentBeginOverlap(Box)
  (params (OverlappedComponent :type Primitive%20Component%20Object%20Reference) (OtherActor :type Actor%20Object%20Reference) (OtherComp :type Primitive%20Component%20Object%20Reference) (OtherBodyIndex :type Integer) (bFromSweep :type Boolean) (SweepResult :type Hit%20Result%20Structure%20%28by%20ref%29))
  (if (not (== OtherActor (Components|GetOwner)))
    (CallFunction|SendGameplayEvent OtherActor "(TagName=\"Gameplay.Combat.Damage.HitByProjectile\")" "/Game/_WhatYouPaidFor_RenameMe/Blueprints/Objects/Damages/BP_Payload_Damage_Arrow.BP_Payload_Damage_Arrow_C")
    (Actor|DestroyActor)))

(event EventBeginPlay
  (CallFunction|SetVelocity))

(event Collision|EventActorBeginOverlap
  (params (OtherActor :type Actor%20Object%20Reference)))

(event EventTick
  (params (DeltaSeconds :type Float%20%28single-precision%29)))

(fn ConstructionScript)

(fn SetVelocity
  (bind _projectilemovement (Variables|Default|GetProjectileMovement))
  (Variables|/Script/Engine.MovementComponent|SetVelocity _projectilemovement (* (Math|Vector|GetUnitDirection(Vector) (Transformation|GetActorLocation) (Transformation|GetActorLocation (Game|Player|GetPlayerPawn 0))) (Variables|/Script/Engine.ProjectileMovementComponent|GetInitialSpeed _projectilemovement))))