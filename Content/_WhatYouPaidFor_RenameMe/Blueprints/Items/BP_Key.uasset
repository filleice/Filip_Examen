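; BP_Key is a pickup key item that the player collects by walking into its sphere.
; When the overlapping actor is the player character, it plays a pickup sound at its location and applies its configurable status tag to the player.
; It then adds the key's UI icon and destroys itself.
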(event OnComponentBeginOverlap(Sphere)
  (params (OverlappedComponent :type Primitive%20Component%20Object%20Reference) (OtherActor :type Actor%20Object%20Reference) (OtherComp :type Primitive%20Component%20Object%20Reference) (OtherBodyIndex :type Integer) (bFromSweep :type Boolean) (SweepResult :type Hit%20Result%20Structure%20%28by%20ref%29))
  (bind _returnvalue (Game|GetPlayerCharacter 0))
  (if (== OtherActor _returnvalue)
    (Audio|PlaySoundatLocation (Variables|Key|Settings|GetPickupSound) (Transformation|GetActorLocation) "0, 0, 0" 1.0 1.0 0.0 0 0 0 0)
    (CallFunction|ApplyStatustoActor _returnvalue true (Variables|Key|Settings|GetStatusThisKeyGIves))
    (CallFunction|AddtoIcons (Variables|Key|Settings|GetKeyIconUI))
    (Actor|DestroyActor)))

(event EventBeginPlay)

(event Collision|EventActorBeginOverlap
  (params (OtherActor :type Actor%20Object%20Reference)))

(event EventTick
  (params (DeltaSeconds :type Float%20%28single-precision%29)))

(fn ConstructionScript)