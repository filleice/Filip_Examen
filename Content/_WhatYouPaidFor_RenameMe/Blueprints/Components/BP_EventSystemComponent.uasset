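; Event system component that routes gameplay-tag events, with a payload and optional object, to registered receiver objects.
; WaitMultipleEvents adds a receiver to a map of receiver lists keyed by tag, while WaitForEvent adds a tag without a receiver.
; ReceiveEvent calls ReceiveEventMessage on receivers under every matching key, including parent tags through non-exact matching.
; Both StopWaiting functions remove whole tag entries, dropping all their receivers.
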(event EventBeginPlay)

(event EventTick
  (params (DeltaSeconds :type Float%20%28single-precision%29)))

(fn ReceiveEvent
  (params (GameplayTag :type Gameplay%20Tag%20Structure) (Payload :type BP%20Payload%20Base%20Class%20Reference) (OptionalObject :type Object%20Object%20Reference))
  (bind _gameplayeventcallbacks (Variables|Default|GetGameplayEventCallbacks))
  (bind _keys (Utilities|Map|Keys _gameplayeventcallbacks))
  (for _array_element _keys
    (if (GameplayTags|MatchesTag GameplayTag _array_element)
      (for _array_element_2 (Utilities|Struct|BreakS_GameplayEventCallbacks (.Value (Utilities|Map|Find _gameplayeventcallbacks _array_element)))
        (Class|BIEventReceiver|ReceiveEvent(Message) _array_element_2 GameplayTag Payload OptionalObject)))))

(fn WaitforEvent
  (params (Tag :type Gameplay%20Tag%20Structure))
  (Utilities|Map|Add :TargetMap (Variables|Default|GetGameplayEventCallbacks) :Key Tag))

(fn StopWaitingforEvent
  (params (Tag :type Gameplay%20Tag%20Structure))
  (Utilities|Map|Remove (Variables|Default|GetGameplayEventCallbacks) Tag))

(fn WaitMultipleEvents
  (params (EventReceiver :type Object%20Object%20Reference%20%28by%20ref%29) (Tags :type Gameplay%20Tag%20Container%20Structure))
  (bind _gameplayeventcallbacks (Variables|Default|GetGameplayEventCallbacks))
  (Utilities|IsValid EventReceiver
    (:Is%20Valid
      (for _array_element (GameplayTags|BreakGameplayTagContainer Tags)
        (if (.ReturnValue (Utilities|Map|Find _gameplayeventcallbacks _array_element))
          (Utilities|Array|Add (Utilities|Struct|BreakS_GameplayEventCallbacks (.Value (Utilities|Map|Find _gameplayeventcallbacks _array_element))) EventReceiver)
          (else
            (Utilities|Map|Add _gameplayeventcallbacks _array_element (Utilities|Struct|MakeS_GameplayEventCallbacks (Utilities|Array|MakeArray EventReceiver)))))))))

(fn StopWaitingMultipleEvents
  (params (Tags :type Gameplay%20Tag%20Container%20Structure))
  (for _array_element (GameplayTags|BreakGameplayTagContainer Tags)
    (Utilities|Map|Remove (Variables|Default|GetGameplayEventCallbacks) _array_element)))