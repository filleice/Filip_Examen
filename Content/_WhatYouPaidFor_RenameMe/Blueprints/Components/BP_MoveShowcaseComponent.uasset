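; Actor component that animates its owner for showcase purposes by spinning it and moving it back and forth.
; On BeginPlay it normalizes the rotation direction and caches the owner's start location.
; Each tick it adds world rotation along that direction, scaled by speed and delta time.
; It also lerps the location between the start and an offset using a time-based sine wave, without sweeping.
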(event EventBeginPlay
  (Variables|Default|SetRotationDirection (Math|Vector|Normalize (Variables|Default|GetRotationDirection)))
  (Variables|Default|SetStartLocation (Transformation|GetActorLocation (Components|GetOwner))))

(event EventTick
  (params (DeltaSeconds :type Float%20%28single-precision%29))
  (CallFunction|RotateActor DeltaSeconds)
  (CallFunction|MoveActor))

(fn RotateActor
  (params (InputPin :type Float%20%28single-precision%29))
  (bind _rotationdirection (Variables|Default|GetRotationDirection))
  (bind _rotationspeed (Variables|Default|GetRotationSpeed))
  (Class|Actor|AddActorWorldRotation (Components|GetOwner) (Math|Rotator|MakeRotator (* InputPin (.x _rotationdirection) _rotationspeed) (* InputPin (.y _rotationdirection) _rotationspeed) (* InputPin (.z _rotationdirection) _rotationspeed))))

(fn MoveActor
  (bind _startlocation (Variables|Default|GetStartLocation))
  (Transformation|SetActorLocation (Components|GetOwner) (Math|Vector|Lerp(Vector) _startlocation (+ _startlocation (Variables|Default|GetLocationDelta)) (* (+ (Math|Trig|Sin(Radians) (* (Utilities|Time|GetTimeSeconds) (Variables|Default|GetMoveSpeed))) 1.0) 0.5)) false false))