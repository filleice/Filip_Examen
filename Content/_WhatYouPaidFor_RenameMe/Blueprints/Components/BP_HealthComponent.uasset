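; BP_HealthComponent is an actor component that tracks its owner's health through tag-based gameplay events.
; On BeginPlay it fills health to max and, if the owner has an event component, listens for damage ModifyHealth events.
; Each damage payload's class-default value is subtracted, clamped at zero but not capped to MaxHealth.
; It then sends a health-changed event to the owner, plus a no-health event at zero.
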(event EventBeginPlay
  (bind _returnvalue (Components|GetOwner))
  (Variables|Default|SetCurrentHealth (Variables|Default|GetMaxHealth))
  (if (.bSuccess (CallFunction|GetEventComponent _returnvalue))
    (CallFunction|StartWaitingMultipleEvents _returnvalue self "(GameplayTags=((TagName=\"Gameplay.Combat.Damage.ModifyHealth\")))")))

(event EventTick
  (params (DeltaSeconds :type Float%20%28single-precision%29)))

(event EventEvent
  (params (Tag :type Gameplay%20Tag%20Structure) (Payload :type BP%20Payload%20Base%20Class%20Reference) (OptionalObject :type Object%20Object%20Reference))
  (CallFunction|OnReceiveDamage Tag Payload))

(fn OnReceiveDamage
  (params (GameplayTag :type Gameplay%20Tag%20Structure) (Payload :type BP%20Payload%20Base%20Class%20Reference))
  (bind _asbp_payload_damage_base (Utilities|Casting|CastToBP_Payload_Damage_BaseClass Payload))
  (Variables|Default|SetCurrentHealth (Math|Integer|Clamp(Integer) (- (Variables|Default|GetCurrentHealth) (Utilities|GetClassDefaults _asbp_payload_damage_base)) 0 9999999))
  (CallFunction|OnHealthChanged))

(fn OnHealthChanged
  (CallFunction|SendGameplayEvent (Components|GetOwner) "(TagName=\"Gameplay.Combat.Health.Changed\")" 0 self)
  (if (<= (Variables|Default|GetCurrentHealth) 0)
    (CallFunction|SendGameplayEvent (Components|GetOwner) "(TagName=\"Gameplay.Combat.Health.NoHealth\")")))