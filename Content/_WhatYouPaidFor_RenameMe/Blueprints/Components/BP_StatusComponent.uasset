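; BP_StatusComponent is a component that tracks status gameplay tags with a count for each.
; ModifyStatusTag increments or decrements a tag's count in the CurrentTags map and removes it at zero, so stacked applications work like reference counting.
; AddMultipleStatusTags adds every tag in a container through that function.
; GetOwnedTags returns the map's keys as a gameplay tag container.
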(fn ModifyStatusTag
  (params (ToAdd :type Boolean) (StatusTag :type Gameplay%20Tag%20Structure))
  (bind _currenttags (Variables|Default|GetCurrentTags))
  (bind (_value _returnvalue) (Utilities|Map|Find _currenttags StatusTag))
  (if ToAdd
    (Utilities|FlowControl|Sequence
      (:then_0
        (if _returnvalue
          (bind _output_get (LocalVariables|SetCurrentValue _value))
          (Utilities|Map|Add _currenttags StatusTag (+ _output_get 1))
          (else
            (Utilities|Map|Add _currenttags StatusTag 1)))))
    (elif _returnvalue
      (bind _output_get_2 (LocalVariables|SetCurrentValue _value))
      (Utilities|Map|Add _currenttags StatusTag (- _output_get_2 1))
      (if (<= (- _output_get_2 1) 0)
        (Utilities|Map|Remove _currenttags StatusTag)))))

(fn GetOwnedTags
  (bind _keys (Utilities|Map|Keys (Variables|Default|GetCurrentTags)))
  (return (GameplayTags|MakeGameplayTagContainerfromArray _keys)))

(fn AddMultipleStatusTags
  (params (Statuses :type Gameplay%20Tag%20Container%20Structure))
  (for _array_element (GameplayTags|BreakGameplayTagContainer Statuses)
    (CallFunction|ModifyStatusTag true _array_element)))