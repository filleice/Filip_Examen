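; Weapon mesh component that performs melee hit detection during attack animations and sends damage gameplay events to the actors it hits.
; It listens on its owner for attack collision Start and End tags to toggle tick and manage the ignore list.
; Each tick it box-traces from last frame's offset position to the current one, covering the swing between frames.
; Hit actors receive an explosion effect and are ignored until End; traces draw debug shapes.
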(event EventBeginPlay
  (CallFunction|StartWaitingMultipleEvents (Components|GetOwner) self "(GameplayTags=((TagName=\"Animation.Combat.Attack.Collision\")))"))

(event EventTick
  (params (DeltaSeconds :type Float%20%28single-precision%29))
  (CallFunction|PerformAttackTrace))

(event EventEvent
  (params (Tag :type Gameplay%20Tag%20Structure) (Payload :type BP%20Payload%20Base%20Class%20Reference))
  (bind _actors_to_ignore (Variables|Default|GetActors%20to%20Ignore))
  (|SwitchGameplayTag Tag
    (:Animation.Combat.Attack.Collision.Start
      (Components|Tick|SetComponentTickEnabled true)
      (Utilities|Array|Add _actors_to_ignore (Components|GetOwner))
      (CallFunction|SetNewLocationLastFrame))
    (:Animation.Combat.Attack.Collision.End
      (Components|Tick|SetComponentTickEnabled false)
      (Utilities|Array|Clear _actors_to_ignore))))

(fn PerformAttackTrace
  (bind _outhits (Class|KismetSystemLibrary|BoxTraceMulti (Variables|Default|GetLocationLastFrame) (CallFunction|GetLocationWIthOffset) (Variables|WeaponInfo|GetHalf%20Size) (Transformation|GetWorldRotation) "TraceTypeQuery3" false (Variables|Default|GetActors%20to%20Ignore) "ForDuration" true))
  (Utilities|FlowControl|Sequence
    (:then_0
      (for _array_element _outhits
        (CallFunction|SendGameplayEvent (.HitActor (Collision|BreakHitResult _array_element)) "(TagName=\"Gameplay.Combat.Damage\")" (Variables|Default|GetDamageType))
        (Utilities|Array|Add (Variables|Default|GetActors%20to%20Ignore) (.HitActor (Collision|BreakHitResult _array_element)))
        (Effects|SpawnEmitteratLocation "/Game/StarterContent/Particles/P_Explosion.P_Explosion" (.ImpactPoint (Collision|BreakHitResult _array_element)) "0, 0, 0" "0.300000,0.300000,0.300000")))
    (:then_1
      (CallFunction|SetNewLocationLastFrame))))

(fn SetNewLocationLastFrame
  (Variables|Default|SetLocationLastFrame (CallFunction|GetLocationWIthOffset)))

(fn GetLocationWIthOffset
  (return (+ (Transformation|GetWorldLocation) (Math|Vector|RotateVector (Variables|Default|GetOffset) (Transformation|GetWorldRotation)))))